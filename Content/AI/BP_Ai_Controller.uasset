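; BP_Ai_Controller is an AI controller that runs BT_Basic and seeds its blackboard with starting Health and IsDead values.
; Perception updates pass the sensed actor through IsEnemyTeam to SetTargetActor, which writes the TargetActor blackboard key, with helper functions to read it back.
; IsEnemyTeam always returns false or stops on a failed cast, leaving its Team comparison unwired, so perception never sets a target.
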(event `self.ReceiveBeginPlay`
  (bind _returnvalue (`AIBlueprintHelperLibrary.GetBlackboard` self))
  (`self.RunBehaviorTree` "/Game/AI/BT_Basic.BT_Basic")
  (`BlackboardComponent.SetValueAsFloat` _returnvalue "Health" 100.0)
  (`BlackboardComponent.SetValueAsBool` _returnvalue "IsDead" false))

(event `self.AIPerception.OnTargetPerceptionUpdated`
  (params (Actor :type "Actor Object Reference") (Stimulus :type "AIStimulus Structure"))
  (bind (_isenemyteam _enemyai) (`self.IsEnemyTeam?` Actor))
  (if _isenemyteam
    (`self.SetTargetActor` _enemyai)))

(fn `GetTargetActor`
  (returns (TargetActor :type "/Game/AI/BP_AI_Character Object Reference"))
  (bind _asbp_ai_character (cast `/Game/AI/BP_AI_Character` (`BlackboardComponent.GetValueAsObject` (`AIBlueprintHelperLibrary.GetBlackboard` self) "TargetActor")))
  (return _asbp_ai_character))

(fn `IsEnemyTeam?`
  (params (Enemy :type "Object Object Reference"))
  (returns (ISEnemyTeam :type Boolean) (EnemyAI :type "/Game/AI/BP_AI_Character Object Reference"))
  (bind _asbp_ai_character (cast `/Game/AI/BP_AI_Character` Enemy))
  (return false null))

(fn `IsTargetActorSet`
  (returns (TargetActor :type "/Game/AI/BP_AI_Character Object Reference") (IsTargetActorSet :type Boolean))
  (bind _returnvalue (`BlackboardComponent.GetValueAsObject` (`AIBlueprintHelperLibrary.GetBlackboard` self) "TargetActor"))
  (bind _asbp_ai_character (cast `/Game/AI/BP_AI_Character` _returnvalue))
  (return _asbp_ai_character (`KismetSystemLibrary.IsValid` _returnvalue)))

(fn `SetTargetActor`
  (params (TheTargetActor :type "/Game/AI/BP_AI_Character Object Reference"))
  (returns (TargetActor :type "/Game/AI/BP_AI_Character Object Reference"))
  (`BlackboardComponent.SetValueAsObject` (`AIBlueprintHelperLibrary.GetBlackboard` self) "TargetActor" TheTargetActor)
  (return TheTargetActor))

(fn `UserConstructionScript`)